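; BP_LightSwitch is a light switch that controls a group of BP_InteractiveLight actors sharing a tag.
; On BeginPlay it gathers every interactive light matching LightTag into LightObjects, then calls SwitchLights if IsOn is false.
; SwitchLights loops over the cached lights and calls SwitchLight on each; nothing else in this Blueprint triggers it.
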(event EventBeginPlay
  (bind _outactors (Actor|GetAllActorsOfClasswithTag "/Game/DEV23_FinalProject/Blueprints/BP_InteractiveLight.BP_InteractiveLight_C" (Variables|Default|GetLightTag)))
  (Variables|Default|SetLightObjects _outactors)
  (if (not (Variables|Default|GetisOn))
    (CallFunction|SwitchLights)))

(event Collision|EventActorBeginOverlap
  (params (OtherActor :type Actor%20Object%20Reference)))

(event EventTick
  (params (DeltaSeconds :type Float%20%28single-precision%29)))

(fn ConstructionScript)

(fn SwitchLights
  (for _array_element (Variables|Default|GetLightObjects)
    (Default|SwitchLight _array_element)))