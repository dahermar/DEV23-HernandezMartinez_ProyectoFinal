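; BP_EnemyGenerator is a destructible enemy spawner actor.
; AnyDamage reduces Health while it is alive; at zero it clears IsAlive, reveals its particles and plays an explosion sound.
; The GenerateEnemy event spawns a BP_EnemyAndroid at an offset from its static mesh while alive, with no caller in this graph.
; Code to pass the generator's first tag to the spawned android is disconnected, so it never runs.
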(event Custom|Generate%20Enemy
  (if (Variables|Default|GetisAlive)
    ;[1 1 1] Conectar para que funcione
    (bind _returnvalue (Game|SpawnActorfromClass "/Game/DEV23_FinalProject/Blueprints/BP_EnemyAndroid.BP_EnemyAndroid_C" (Math|Transform|MakeTransform (+ (Transformation|GetWorldLocation (Variables|Default|GetStaticMesh)) "0.000000,100.000000,50.000000") "0, 0, 0" "1.000000,1.000000,1.000000") "Undefined" "MultiplyWithRoot" 0 0))))

(event EventBeginPlay)

(event Collision|EventActorBeginOverlap
  (params (OtherActor :type Actor%20Object%20Reference)))

(event EventTick
  (params (DeltaSeconds :type Float%20%28single-precision%29)))

(event Game|Damage|EventAnyDamage
  (params (Damage :type Float%20%28single-precision%29) (DamageType :type Damage%20Type%20Object%20Reference) (InstigatedBy :type Controller%20Object%20Reference) (DamageCauser :type Actor%20Object%20Reference))
  (if (Variables|Default|GetisAlive)
    (bind _output_get (Variables|Default|SetHealth (- (Variables|Default|GetHealth) Damage)))
    (if (<= _output_get 0.0)
      (Variables|Default|SetisAlive false)
      (Rendering|SetVisibility (Variables|Default|GetParticles) true false)
      (Audio|PlaySoundatLocation "/Game/StarterContent/Audio/Explosion_Cue.Explosion_Cue" (Transformation|GetActorLocation) "0, 0, 0" 1.0 2.0 0.0 0 0 0 0))))

(fn ConstructionScript)