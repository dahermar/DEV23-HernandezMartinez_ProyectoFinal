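; Enemy android character that patrols, shoots the player and can be stunned, damaged, killed instantly by headshot or taken down from behind.
; At BeginPlay it adds a weapon component and builds a patrol route from EnemyID-tagged path points sorted by PathStep, traversed as a loop or back-and-forth.
; It forwards stun and player light/dark changes to its AI controller.
; Death ragdolls the mesh, timer-delayed for takedowns, and unregisters it from the player.
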(event Custom|Stop%20Shooting
  (if (Variables|Default|GetisAlive)
    (Default|StopShooting (Variables|Default|GetEquipedWeapon))))

(event Custom|Start%20Shooting
  (if (Math|Boolean|ANDBoolean (Variables|Default|GetisAlive) (not (Variables|Default|GetisStunned)) (not (Variables|Default|GetisInTakedown)))
    (Default|StartShooting (Variables|Default|GetEquipedWeapon) (Variables|Default|GetPlayerCharacter))))

(event Custom|Stun
  (bind _enemy_ai_controller (Variables|Default|GetEnemy%20AI%20Controller))
  (Variables|Default|SetisStunned true)
  (Default|BeginStun _enemy_ai_controller)
  (Utilities|FlowControl|Delay 5.0)
  (Variables|Default|SetisStunned false)
  (Default|EndStun _enemy_ai_controller (Variables|Default|GetisPlayerOnLight)))

(event Custom|Player%20Killed
  (CallFunction|StopShooting))

(event Custom|Player%20on%20Dark
  (params (Actor :type Actor%20Object%20Reference))
  (Variables|Default|SetisPlayerOnLight false)
  (if (not (Variables|Default|GetisStunned))
    (Default|ChangetoDark (Variables|Default|GetEnemy%20AI%20Controller) Actor)))

(event Custom|Player%20on%20Light
  (Variables|Default|SetisPlayerOnLight true)
  (if (not (Variables|Default|GetisStunned))
    (Default|ChangetoLight (Variables|Default|GetEnemy%20AI%20Controller))))

(event EventBeginPlay
  (bind _todelete (Variables|Default|GettoDelete))
  (bind _returnvalue (AddComponent|AddBPEnemyWeaponComponent false))
  (Variables|Default|SetEquipedWeapon _returnvalue)
  (Variables|Default|SetEnemy%20AI%20Controller (.AsBP%20Enemy%20Android%20Controller (Utilities|Casting|CastToBP_EnemyAndroidController (AI|GetAIController self))))
  (Variables|Default|SetPlayerCharacter (.AsBP%20My%20Third%20Person%20Character (Utilities|Casting|CastToBP_MyThirdPersonCharacter (Game|GetPlayerCharacter 0))))
  ;[1 1 1] Creación del camino de patrulla en el orden indicado por la variable PathStep de los ParthPoint. Es encesario ordenarlos ya que al hacer get Actors of Class no aparecen ordenados por defecto
  (bind _outactors (Actor|GetAllActorsOfClasswithTag "/Game/DEV23_FinalProject/Blueprints/BP_PathPoint.BP_PathPoint_C" (Variables|Default|GetEnemyID)))
  (while (> (Utilities|Array|Length _outactors) 0)
    (for (_array_element _array_index) _outactors
      (if (== (Variables|/Game/DEV23_FinalProject/Blueprints/BP_PathPoint.BP_PathPoint_C|GetPathStep _array_element) (Variables|Default|GetpathStepIndex))
        (Utilities|Array|Add (Variables|Default|GetPathPositions) (Transformation|GetActorLocation _array_element))
        (Utilities|Array|Add (Variables|Default|GettoDelete) _array_index)))
    (Math|Integer|IncrementInt (Variables|Default|GetpathStepIndex)
      (:%20%20
        (bind _arrayelement (Utilities|Array|ReverseforEachLoop _todelete)
          (:LoopBody
            (Utilities|Array|RemoveIndex _outactors _arrayelement))
          (:Completed
            (Utilities|Array|Clear _todelete))))))
  (Variables|Default|SetpathStepIndex -1)
  (Variables|Default|SetnumberOfSteps (Utilities|Array|Length (Variables|Default|GetPathPositions))))

(event EventTakeDamage
  (params (Damage :type Float%20%28double-precision%29) (HitBoneName :type Name :default "None"))
  (if (Variables|Default|GetisAlive)
    (if (== HitBoneName (Variables|Default|GetHeadBoneName))
      (CallFunction|Die :!label _label)
      (else
        (bind _output_get (Variables|Default|SetHealth (- (Variables|Default|GetHealth) Damage)))
        (if (<= _output_get 0.0)
          (goto _label))))))

(event Game|Damage|EventAnyDamage
  (params (Damage :type Float%20%28single-precision%29) (DamageType :type Damage%20Type%20Object%20Reference) (InstigatedBy :type Controller%20Object%20Reference) (DamageCauser :type Actor%20Object%20Reference))
  (if (Variables|Default|GetisAlive)
    (bind _output_get (Variables|Default|SetHealth (- (Variables|Default|GetHealth) Damage)))
    (if (<= _output_get 0.0)
      (CallFunction|Die))))

(fn ConstructionScript)

(fn Die
  (Variables|Default|SetisAlive false)
  (Components|DestroyComponent (Variables|Default|GetTakedownArea))
  (Collision|SetCollisionEnabled (Variables|Collision|GetCapsuleComponent) "NoCollision")
  (Physics|SetSimulatePhysics (Variables|Character|GetMesh) true)
  (Pawn|Components|CharacterMovement|SetMovementMode (Variables|Character|GetCharacterMovement) "MOVE_None" 0)
  (Default|StopShooting (Variables|Default|GetEquipedWeapon))
  (Default|RemoveEnemy (Variables|Default|GetPlayerCharacter) self))

(fn NextPatrolLocation
  (switch int (Variables|Default|GetPathMode)
    (:Default
      _)
    (:0
      ;[1 1 1] Patrullaje circular
      (bind _result (Math|Integer|IncrementInt (Variables|Default|GetpathStepIndex))
        (:%20%20
          (if (< _result (Variables|Default|GetnumberOfSteps))
            _
            (else
              (Variables|Default|SetpathStepIndex 0)))
          (return (Utilities|Array|Get(acopy) (Variables|Default|GetPathPositions) (Variables|Default|GetpathStepIndex))))))
    (:1
      _))
  ;[1 1 1] Patrullaje con camino de retorno
  (Variables|Default|SetpathStepIndex (+ (Variables|Default|GetPathDirection) (Variables|Default|GetpathStepIndex)))
  (if (and (>= (Variables|Default|GetpathStepIndex) 0) (< (Variables|Default|GetpathStepIndex) (Variables|Default|GetnumberOfSteps)))
    _
    (else
      (Variables|Default|SetpathStepIndex (- (Variables|Default|GetpathStepIndex) (* (Variables|Default|GetPathDirection) 2)))
      (Variables|Default|SetPathDirection (* -1 (Variables|Default|GetPathDirection)))))
  (return (Utilities|Array|Get(acopy) (Variables|Default|GetPathPositions) (Variables|Default|GetpathStepIndex))))

(fn BackTakedown
  (Variables|Default|SetisInTakedown true)
  (Collision|SetCollisionEnabled (Variables|Collision|GetCapsuleComponent) "NoCollision")
  (Animation|PlayAnimMontage "/Game/DEV23_FinalProject/Animations/Sequences/Takedown/Paired_Knife_Stealth_KidneyAndNeck_Vic_Montage.Paired_Knife_Stealth_KidneyAndNeck_Vic_Montage" 1.0 "None")
  (Utilities|Time|SetTimerbyFunctionName 0 "Die" 2.6)
  (return (Transformation|GetWorldLocation (Variables|Default|GetTakedownAttacker)) (Transformation|GetActorRotation)))