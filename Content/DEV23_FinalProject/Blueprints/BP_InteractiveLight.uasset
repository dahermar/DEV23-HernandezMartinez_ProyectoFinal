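; BP_InteractiveLight is a switchable spotlight actor that notifies overlapping actors when they enter or leave its light.
; Begin and end overlap events send start and end messages to actors implementing BPI_LightOverlap.
; SwitchLight toggles IsOn, which drives spotlight visibility and LightCollision's overlap generation, as does the construction script.
; Both then nudge the collision slightly upward in either state, apparently to refresh overlaps, so repeated toggles accumulate offset.
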(event Collision|EventActorBeginOverlap
  (params (OtherActor :type Actor%20Object%20Reference))
  (if (Utilities|DoesObjectImplementInterface OtherActor "/Game/DEV23_FinalProject/Blueprints/Interfaces/BPI_LightOverlap.BPI_LightOverlap_C")
    (Class|BPILightOverlap|StartLightOverlap(Message) OtherActor)))

(event Collision|EventActorEndOverlap
  (params (OtherActor :type Actor%20Object%20Reference))
  (if (Utilities|DoesObjectImplementInterface OtherActor "/Game/DEV23_FinalProject/Blueprints/Interfaces/BPI_LightOverlap.BPI_LightOverlap_C")
    (Class|BPILightOverlap|EndLightOverlap(Message) OtherActor)))

(fn ConstructionScript
  (bind _ison (Variables|Default|GetIsOn))
  (bind _lightcollision (Variables|Default|GetLightCollision))
  (Rendering|SetVisibility (Variables|Default|GetSpotLight) _ison false)
  (Variables|/Script/Engine.PrimitiveComponent|SetbGenerateOverlapEvents _lightcollision _ison)
  (if _ison
    (Transformation|AddWorldOffset _lightcollision "0.000000,0.000000,0.100000" false false)
    (else
      (Transformation|AddWorldOffset _lightcollision "0.000000,0.000000,0.100000" false false))))

(fn SwitchLight
  (bind _lightcollision (Variables|Default|GetLightCollision))
  (bind _output_get (Variables|Default|SetIsOn (not (Variables|Default|GetIsOn))))
  (Rendering|SetVisibility (Variables|Default|GetSpotLight) _output_get false)
  (Variables|/Script/Engine.PrimitiveComponent|SetbGenerateOverlapEvents _lightcollision _output_get)
  (if _output_get
    (Transformation|AddWorldOffset _lightcollision "0.000000,0.000000,0.100000" false false)
    (else
      (Transformation|AddWorldOffset _lightcollision "0.000000,0.000000,0.100000" false false))))