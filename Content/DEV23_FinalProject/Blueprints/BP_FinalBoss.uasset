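; Final boss enemy that shoots the player and dies only from a hit on its weak-point bone, ending the game.
; BeginPlay adds a high-damage weapon component and a small cube marking the WeakPoint socket.
; Player light/dark events switch its AI controller state, and NextPatrolLocation supplies looping or back-and-forth patrol points.
; Death ragdolls the mesh and stops shooting, then after a delay pauses the game and shows the game-end widget.
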(event Custom|Stop%20Shooting
  (if (Variables|Default|GetisAlive)
    (Default|StopShooting (Variables|Default|GetEquipedWeapon))))

(event Custom|Start%20Shooting
  (if (Variables|Default|GetisAlive)
    (Default|StartShooting (Variables|Default|GetEquipedWeapon) (Variables|Default|GetPlayerCharacter))))

(event Custom|Player%20Killed
  (CallFunction|StopShooting))

(event Custom|Player%20on%20Dark
  (params (Actor :type Actor%20Object%20Reference))
  (Variables|Default|SetisPlayerOnLight false)
  (Default|ChangetoDark (Variables|Default|GetEnemy%20AI%20Controller) Actor))

(event Custom|Player%20on%20Light
  (Variables|Default|SetisPlayerOnLight true)
  (Default|ChangetoLight (Variables|Default|GetEnemy%20AI%20Controller)))

(event EventBeginPlay
  (bind _returnvalue (AddComponent|AddBPEnemyWeaponComponent false))
  (bind _output_get (Variables|Default|SetEquipedWeapon _returnvalue))
  (Variables|/Game/DEV23_FinalProject/Blueprints/Weapons/BP_EnemyWeapon_Component.BP_EnemyWeapon_Component_C|SetDamage _output_get 2e+02)
  (Variables|Default|SetEnemy%20AI%20Controller (.AsBP%20Enemy%20Android%20Controller (Utilities|Casting|CastToBP_EnemyAndroidController (AI|GetAIController self))))
  (Variables|Default|SetPlayerCharacter (.AsBP%20My%20Third%20Person%20Character (Utilities|Casting|CastToBP_MyThirdPersonCharacter (Game|GetPlayerCharacter 0))))
  (bind _returnvalue_2 (AddComponent|AddStaticMeshComponent false (Math|Transform|MakeTransform "0, 0, 0" "0, 0, 0" "0.050000,0.010000,0.050000")))
  (Components|StaticMesh|SetStaticMesh _returnvalue_2 "/Engine/EngineMeshes/Cube.Cube")
  (Rendering|Material|SetMaterial _returnvalue_2 0 "/Engine/VREditor/LaserPointer/LaserPointerMaterial.LaserPointerMaterial")
  (Collision|SetCollisionEnabled _returnvalue_2 "NoCollision")
  (Transformation|AttachComponentToComponent _returnvalue_2 (Variables|Character|GetMesh) "WeakPoint" "KeepRelative" "KeepRelative" "KeepRelative" true)
  (CallFunction|PlayeronLight))

(event EventTakeDamage
  (params (Damage :type Float%20%28double-precision%29) (HitBoneName :type Name :default "None"))
  (if (Variables|Default|GetisAlive)
    (if (== HitBoneName (Variables|Default|GetWeakPointName))
      (CallFunction|Die)
      (Utilities|FlowControl|Delay 1.0)
      (Game|SetGamePaused true)
      (Viewport|RemoveAllWidgets)
      (bind _returnvalue (UserInterface|CreateWidget "/Game/DEV23_FinalProject/Widgets/WB_GameEnd.WB_GameEnd_C"))
      (UserInterface|Viewport|AddtoViewport _returnvalue 0))))

(fn ConstructionScript)

(fn Die
  (Variables|Default|SetisAlive false)
  (Collision|SetCollisionEnabled (Variables|Collision|GetCapsuleComponent) "NoCollision")
  (Physics|SetSimulatePhysics (Variables|Character|GetMesh) true)
  (Pawn|Components|CharacterMovement|SetMovementMode (Variables|Character|GetCharacterMovement) "MOVE_None" 0)
  (Default|StopShooting (Variables|Default|GetEquipedWeapon)))

(fn NextPatrolLocation
  (switch int (Variables|Default|GetPathMode)
    (:Default
      _)
    (:0
      ;[1 1 1] Patrullaje circular
      (bind _result (Math|Integer|IncrementInt (Variables|Default|GetpathStepIndex))
        (:%20%20
          (if (< _result (Variables|Default|GetnumberOfSteps))
            _
            (else
              (Variables|Default|SetpathStepIndex 0)))
          (return (Utilities|Array|Get(acopy) (Variables|Default|GetPathPositions) (Variables|Default|GetpathStepIndex))))))
    (:1
      _))
  ;[1 1 1] Patrullaje con camino de retorno
  (Variables|Default|SetpathStepIndex (+ (Variables|Default|GetPathDirection) (Variables|Default|GetpathStepIndex)))
  (if (and (>= (Variables|Default|GetpathStepIndex) 0) (< (Variables|Default|GetpathStepIndex) (Variables|Default|GetnumberOfSteps)))
    _
    (else
      (Variables|Default|SetpathStepIndex (- (Variables|Default|GetpathStepIndex) (* (Variables|Default|GetPathDirection) 2)))
      (Variables|Default|SetPathDirection (* -1 (Variables|Default|GetPathDirection)))))
  (return (Utilities|Array|Get(acopy) (Variables|Default|GetPathPositions) (Variables|Default|GetpathStepIndex))))