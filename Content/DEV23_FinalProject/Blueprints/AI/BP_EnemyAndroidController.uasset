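; AI controller for the enemy android that runs its behavior tree and turns sight and hearing into blackboard values.
; Separate light and dark sight perception components are toggled as lighting changes.
; Sight sets the player and line-of-sight keys, while lost sight or a heard sound sets the move destination.
; Stun disables all senses and clears those targets until it ends, and player invisibility switches off both sight components.
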(event OnTargetPerceptionUpdated(AIPerception)
  (params (Actor :type Actor%20Object%20Reference) (Stimulus :type AI%20Stimulus%20Structure))
  (bind (_age _expirationage _strength _stimuluslocation _receiverlocation _tag _bsuccessfullysensed) (Utilities|Struct|BreakAIStimulus Stimulus))
  (bind _returnvalue (Class|AIPerceptionSystem|GetSenseClassforStimulus Stimulus))
  (if (== _returnvalue "/Script/AIModule.AISense_Sight")
    (CallFunction|HandleSightPerception Actor _bsuccessfullysensed)
    (elif (== _returnvalue "/Script/AIModule.AISense_Hearing")
      (CallFunction|HandleHearingPerception _stimuluslocation))))

(event OnTargetPerceptionUpdated(AIPerceptionSightLight)
  (params (Actor :type Actor%20Object%20Reference) (Stimulus :type AI%20Stimulus%20Structure))
  (Utilities|Casting|CastToBP_MyThirdPersonCharacter Actor)
  (CallFunction|HandleSightPerception Actor (.bSuccessfullySensed (Utilities|Struct|BreakAIStimulus Stimulus))))

(event OnTargetPerceptionUpdated(AIPerceptionSightDark)
  (params (Actor :type Actor%20Object%20Reference) (Stimulus :type AI%20Stimulus%20Structure))
  (Utilities|Casting|CastToBP_MyThirdPersonCharacter Actor)
  (CallFunction|HandleSightPerception Actor (.bSuccessfullySensed (Utilities|Struct|BreakAIStimulus Stimulus))))

(event Custom|Change%20to%20Dark
  (params (Actor :type Actor%20Object%20Reference))
  (Class|AIPerceptionComponent|SetSenseEnabled (Variables|Default|GetAIPerceptionSightLight) "/Script/AIModule.AISense_Sight" false)
  (Class|AIPerceptionComponent|SetSenseEnabled (Variables|Default|GetAIPerceptionSightDark) "/Script/AIModule.AISense_Sight" true)
  (if (ScalableFloat|GetValueasBool (Variables|Default|GetBlackboard) (Utilities|Name|MakeLiteralName "HasLineOfSight"))
    (CallFunction|HandleSightPerception Actor false)))

(event Custom|Change%20To%20Light
  (Class|AIPerceptionComponent|SetSenseEnabled (Variables|Default|GetAIPerceptionSightDark) "/Script/AIModule.AISense_Sight" false)
  (Class|AIPerceptionComponent|SetSenseEnabled (Variables|Default|GetAIPerceptionSightLight) "/Script/AIModule.AISense_Sight" true))

(event Custom|EndStun
  (params (isOnLight :type Boolean))
  (Class|AIPerceptionComponent|SetSenseEnabled (Variables|Default|GetAIPerception) "/Script/AIModule.AISense_Hearing" true)
  (if isOnLight
    (Class|AIPerceptionComponent|SetSenseEnabled (Variables|Default|GetAIPerceptionSightLight) "/Script/AIModule.AISense_Sight" true)
    (else
      (Class|AIPerceptionComponent|SetSenseEnabled (Variables|Default|GetAIPerceptionSightDark) "/Script/AIModule.AISense_Sight" true)))
  (AI|Components|Blackboard|SetValueasBool (Variables|Default|GetBlackboard) (Utilities|Name|MakeLiteralName "IsStunned") false))

(event Custom|BeginStun
  (Class|AIPerceptionComponent|SetSenseEnabled (Variables|Default|GetAIPerception) "/Script/AIModule.AISense_Hearing" false)
  (Class|AIPerceptionComponent|SetSenseEnabled (Variables|Default|GetAIPerceptionSightLight) "/Script/AIModule.AISense_Sight" false)
  (Class|AIPerceptionComponent|SetSenseEnabled (Variables|Default|GetAIPerceptionSightDark) "/Script/AIModule.AISense_Sight" false)
  (CallFunction|ClearBlackboard)
  (AI|Components|Blackboard|SetValueasBool (Variables|Default|GetBlackboard) (Utilities|Name|MakeLiteralName "IsStunned") true))

(event Custom|Player%20Invisible
  (Class|AIPerceptionComponent|SetSenseEnabled (Variables|Default|GetAIPerceptionSightLight) "/Script/AIModule.AISense_Sight" false)
  (Class|AIPerceptionComponent|SetSenseEnabled (Variables|Default|GetAIPerceptionSightDark) "/Script/AIModule.AISense_Sight" false))

(event EventPossess
  (params (PossessedPawn :type Pawn%20Object%20Reference))
  (AI|RunBehaviorTree "/Game/DEV23_FinalProject/Blueprints/AI/BT_EnemyAndroid.BT_EnemyAndroid")
  (Class|AIPerceptionComponent|SetSenseEnabled (Variables|Default|GetAIPerceptionSightDark) "/Script/AIModule.AISense_Sight" true))

(fn ConstructionScript)

(fn HandleSightPerception
  (params (Actor :type Actor%20Object%20Reference) (Successfully%20Sensed :type Boolean))
  (bind _blackboard (Variables|Default|GetBlackboard))
  (if Successfully%20Sensed
    (AI|Components|Blackboard|SetValueasObject _blackboard (Utilities|Name|MakeLiteralName "PlayerCharacter") Actor)
    (AI|Components|Blackboard|SetValueasBool _blackboard (Utilities|Name|MakeLiteralName "HasLineOfSight") true)
    (else
      (CallFunction|RemoveLineOfSight Actor))))

(fn HandleHearingPerception
  (params (SoundLocation :type Vector))
  (AI|Components|Blackboard|SetValueasVector (Variables|Default|GetBlackboard) (Utilities|Name|MakeLiteralName "MoveDestiny") SoundLocation))

(fn RemoveLineOfSight
  (params (Actor :type Actor%20Object%20Reference))
  (bind _blackboard (Variables|Default|GetBlackboard))
  (AI|Components|Blackboard|SetValueasBool _blackboard (Utilities|Name|MakeLiteralName "HasLineOfSight") false)
  (AI|Components|Blackboard|SetValueasVector _blackboard (Utilities|Name|MakeLiteralName "MoveDestiny") (Transformation|GetActorLocation Actor)))

(fn ClearBlackboard
  (bind _blackboard (Variables|Default|GetBlackboard))
  (AI|Components|Blackboard|SetValueasBool _blackboard (Utilities|Name|MakeLiteralName "HasLineOfSight") false)
  (AI|Components|Blackboard|ClearValue _blackboard (Utilities|Name|MakeLiteralName "MoveDestiny")))