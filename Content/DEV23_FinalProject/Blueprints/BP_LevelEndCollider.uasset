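; Level exit trigger that opens the next level when the player character overlaps it, optionally requiring a key.
; Before travel, it saves rifle ammo, equipped power and current weapon index to the game instance so they carry over.
; If a needed key is missing, it shows a Spanish HUD prompt asking for the command room card, hidden again when the overlap ends.
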(event Collision|EventActorBeginOverlap
  (params (OtherActor :type Actor%20Object%20Reference))
  (bind _asbp_my_third_person_character (Utilities|Casting|CastToBP_MyThirdPersonCharacter OtherActor))
  (if (Variables|Default|GetneedsKey)
    (if (Variables|/Game/DEV23_FinalProject/Blueprints/BP_MyThirdPersonCharacter.BP_MyThirdPersonCharacter_C|GethasKey _asbp_my_third_person_character)
      (CallFunction|UpdateGameInstance :!label _label)
      (Game|OpenLevel(byName) (Variables|Default|GetNextLevelName))
      (else
        (bind _asthird_person_hud (Utilities|Casting|CastToThirdPersonHUD (HUD|GetHUD (Game|GetPlayerController 0))))
        (Widget|SetVisibility (Variables|/Game/DEV23_FinalProject/Widgets/WB_FirstPersonUI.WB_FirstPersonUI_C|GetDoorText (Variables|/Game/DEV23_FinalProject/Blueprints/ThirdPersonHUD.ThirdPersonHUD_C|GetUIReference _asthird_person_hud)) "Visible")
        (Rendering|Components|TextRender|SetText (Variables|/Game/DEV23_FinalProject/Widgets/WB_FirstPersonUI.WB_FirstPersonUI_C|GetDoorText (Variables|/Game/DEV23_FinalProject/Blueprints/ThirdPersonHUD.ThirdPersonHUD_C|GetUIReference _asthird_person_hud)) "Necesitas la tarjeta de la sala de mando para continuar")))
    (else
      (goto _label))))

(event Collision|EventActorEndOverlap
  (params (OtherActor :type Actor%20Object%20Reference))
  (Utilities|Casting|CastToBP_MyThirdPersonCharacter OtherActor)
  (bind _asthird_person_hud (Utilities|Casting|CastToThirdPersonHUD (HUD|GetHUD (Game|GetPlayerController 0))))
  (Widget|SetVisibility (Variables|/Game/DEV23_FinalProject/Widgets/WB_FirstPersonUI.WB_FirstPersonUI_C|GetDoorText (Variables|/Game/DEV23_FinalProject/Blueprints/ThirdPersonHUD.ThirdPersonHUD_C|GetUIReference _asthird_person_hud)) "Collapsed"))

(fn ConstructionScript)

(fn UpdateGameInstance
  (bind _asbp_my_third_person_character (Utilities|Casting|CastToBP_MyThirdPersonCharacter (Game|GetPlayerCharacter 0)))
  (bind _asbp_my_game_instance (Utilities|Casting|CastToBP_MyGameInstance (Game|GetGameInstance)))
  (Variables|/Game/DEV23_FinalProject/Blueprints/BP_MyGameInstance.BP_MyGameInstance_C|SetRifleAmmo _asbp_my_game_instance (Variables|/Game/DEV23_FinalProject/Blueprints/Weapons/BP_AndroidWeapon_Component.BP_AndroidWeapon_Component_C|GetAmmo (Variables|/Game/DEV23_FinalProject/Blueprints/BP_MyThirdPersonCharacter.BP_MyThirdPersonCharacter_C|GetWeapon%201 _asbp_my_third_person_character)))
  (Variables|/Game/DEV23_FinalProject/Blueprints/BP_MyGameInstance.BP_MyGameInstance_C|SetEquipedPower _asbp_my_game_instance (Variables|/Game/DEV23_FinalProject/Blueprints/BP_MyThirdPersonCharacter.BP_MyThirdPersonCharacter_C|GetEquipedPower _asbp_my_third_person_character))
  (Variables|/Game/DEV23_FinalProject/Blueprints/BP_MyGameInstance.BP_MyGameInstance_C|SetEquiped%20Weapon _asbp_my_game_instance (Variables|/Game/DEV23_FinalProject/Blueprints/BP_MyThirdPersonCharacter.BP_MyThirdPersonCharacter_C|GetCurrentWeaponIndex _asbp_my_third_person_character)))